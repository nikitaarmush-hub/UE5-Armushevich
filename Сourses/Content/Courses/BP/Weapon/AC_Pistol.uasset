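; AC_Pistol is a pistol weapon Blueprint that fires projectiles.
; Its ProjecttileShoot function spawns an actor of ProjectileClass at the MuzzlePoint's world location and rotation, always spawning regardless of collision, and passes the Damage value to it.
; The event graph holds only disabled placeholder events, and the construction script just calls its parent.
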(fn `ProjecttileShoot`
  (bind (_returnvalue_location _returnvalue_rotation) (`KismetMathLibrary.BreakTransform` (`SceneComponent.K2_GetComponentToWorld` (`self.MuzzlePoint`))))
  (`|SpawnActorFromClass` (`self.ProjectileClass`) (`KismetMathLibrary.MakeTransform` _returnvalue_location _returnvalue_rotation) "AlwaysSpawn" "MultiplyWithRoot" null (`self.Damage`) null))

(fn `UserConstructionScript`
  (`parent.UserConstructionScript`))