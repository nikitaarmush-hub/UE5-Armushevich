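; AC_Automatic is a weapon Blueprint whose Shoot event fires both a hitscan trace and a burst of projectiles.
; A CanShoot flag and a Delay limit the fire rate to one shot per cooldown.
; LineShoot traces a short debug-drawn line forward from MuzzlePoint and applies damage to the hit actor.
; ProjecttileShoot spawns a batch of projectiles with random world X and Z offsets, passing each the weapon's Damage.
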(event `self.ReceiveTick`
  (params (DeltaSeconds :type "Float (single-precision)")))

(event `Shoot`
  (if (`self.bCanShoot`)
    (set `self.bCanShoot` false)
    (`KismetSystemLibrary.PrintString` "Fire")
    (`self.LineShoot`)
    (`self.ProjecttileShoot`)
    (`KismetSystemLibrary.Delay` (`self.Coldown`))
    (set `self.bCanShoot` true)))

(fn `LineShoot`
  (bind _muzzlepoint (`self.MuzzlePoint`))
  (bind _returnvalue (`SceneComponent.K2_GetComponentLocation` _muzzlepoint))
  (bind _outhit (`KismetSystemLibrary.LineTraceSingle` :`Start` _returnvalue :`End` (+ _returnvalue (* (`SceneComponent.GetForwardVector` _muzzlepoint) 1000.0)) :`TraceChannel` "TraceTypeQuery1" :`DrawDebugType` "ForDuration"))
  (`GameplayStatics.ApplyDamage` (`.HitActor` (`GameplayStatics.BreakHitResult` _outhit)) (`self.Damage`)))

(fn `ProjecttileShoot`
  (bind _returnvalue (`SceneComponent.K2_GetComponentToWorld` (`self.MuzzlePoint`)))
  (for _ (range 16)
    (`|SpawnActorFromClass` (`self.ProjectileClass`) (`KismetMathLibrary.MakeTransform` (`KismetMathLibrary.MakeVector` (+ (.x (.location _returnvalue)) (`KismetMathLibrary.RandomFloatInRange` 30.0 100.0)) (.y (.location _returnvalue)) (+ (.z (.location _returnvalue)) (`KismetMathLibrary.RandomFloatInRange` 0.0 25.0))) (.rotation _returnvalue)) "AlwaysSpawn" "MultiplyWithRoot" null (`self.Damage`) null)))

(fn `UserConstructionScript`)