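; Player character with mouse-aimed movement, two toggleable cameras, interaction and three switchable weapons.
; Each Tick turns control yaw toward the cursor's intersection with a horizontal plane at the actor, while Enhanced Input drives capsule-relative movement.
; Capsule overlaps store tagged BPI_Interactive targets for the interact action.
; Number keys show or holster pistol, automatic or sniper child actors; firing casts the held one to AC_Automatic and calls Shoot.
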(event `EnhancedInput|/Game/Courses/IA_Courses/IA_Vis`
  (params (ActionValue :type Boolean) (ElapsedSeconds :type "Float (double-precision)") (TriggeredSeconds :type "Float (double-precision)") (InputAction :type "InputAction Object Reference" :default "/Game/Courses/IA_Courses/IA_Vis.IA_Vis"))
  (:`Triggered`
    (`/Engine/EditorBlueprintResources/StandardMacros.FlipFlop`
      (:`A`
        (`ActorComponent.Deactivate` (`self.SecondCamera`))
        (`ActorComponent.Activate` (`self.FirstCamera`) false)
        (set `CameraComponent.bUsePawnControlRotation` true (`self.FirstCamera`))
        (set `CharacterMovementComponent.bOrientRotationToMovement` false (`self.CharacterMovement`))
        (set `self.bUseControllerRotationYaw` true))
      (:`B`
        (`ActorComponent.Deactivate` (`self.FirstCamera`))
        (`ActorComponent.Activate` (`self.SecondCamera`) false)
        (set `CameraComponent.bUsePawnControlRotation` false (`self.FirstCamera`))
        (set `CharacterMovementComponent.bOrientRotationToMovement` true (`self.CharacterMovement`))
        (set `self.bUseControllerRotationYaw` false)))))

(event `self.ReceiveBeginPlay`
  (`self.AddMappingContext`)
  (set `self.GunNow` null))

(event `EnhancedInput|/Game/Courses/IA_Courses/IA_Move`
  (params (ActionValue :type "Vector2D Structure") (ElapsedSeconds :type "Float (double-precision)") (TriggeredSeconds :type "Float (double-precision)") (InputAction :type "InputAction Object Reference" :default "/Game/Courses/IA_Courses/IA_Move.IA_Move"))
  (:`Triggered`
    (`self.Moving` ActionValue_X ActionValue_X ActionValue_Y ActionValue_Y)))

(event `EnhancedInput|/Game/Courses/IA_Courses/IA_Interact`
  (params (ActionValue :type Boolean) (ElapsedSeconds :type "Float (double-precision)") (TriggeredSeconds :type "Float (double-precision)") (InputAction :type "InputAction Object Reference" :default "/Game/Courses/IA_Courses/IA_Interact.IA_Interact"))
  (bind _targetinteractactor (`self.TargetInteractActor`))
  (:`Started`
    (`/Engine/EditorBlueprintResources/StandardMacros.IsValid` _targetinteractactor
      (:`Is Valid`
        (message `/Game/Courses/BP/BPI_Interactive.Interactive` _targetinteractactor self)))))

(event `self.ReceiveTick`
  (params (DeltaSeconds :type "Float (single-precision)"))
  (`self.MouseControllRotation`))

(event `self.CapsuleComponent.OnComponentBeginOverlap`
  (params (OverlappedComponent :type "PrimitiveComponent Object Reference") (OtherActor :type "Actor Object Reference") (OtherComp :type "PrimitiveComponent Object Reference") (OtherBodyIndex :type Integer) (bFromSweep :type Boolean) (SweepResult :type "HitResult Structure (by ref)"))
  (if (and (`KismetSystemLibrary.DoesImplementInterface` OtherActor "/Game/Courses/BP/BPI_Interactive.BPI_Interactive_C") (`ActorComponent.ComponentHasTag` OtherComp "InteractiveTrigger"))
    (set `self.TargetInteractActor` OtherActor)))

(event `self.CapsuleComponent.OnComponentEndOverlap`
  (params (OverlappedComponent :type "PrimitiveComponent Object Reference") (OtherActor :type "Actor Object Reference") (OtherComp :type "PrimitiveComponent Object Reference") (OtherBodyIndex :type Integer))
  (if (`ActorComponent.ComponentHasTag` OtherComp "InteractiveTrigger")
    (if (== OtherActor (`self.TargetInteractActor`))
      (set `self.TargetInteractActor` null))))

(event `EnhancedInput|/Game/Courses/IA_Courses/IA_Shot`
  (params (ActionValue :type Boolean) (ElapsedSeconds :type "Float (double-precision)") (TriggeredSeconds :type "Float (double-precision)") (InputAction :type "InputAction Object Reference" :default "/Game/Courses/IA_Courses/IA_Shot.IA_Shot"))
  ; Shoot
  (:`Started`
    (if (or (or (== (`self.GunNow`) (`self.AC_Pistol`)) (== (`self.GunNow`) (`self.AC_Automatic`))) (== (`self.GunNow`) (`self.AC_Sniper`)))
      (bind _asac_automatic (cast `/Game/Courses/BP/Weapon/AC_Automatic` (`ChildActorComponent.ChildActor` (`self.GunNow`))))
      (`/Game/Courses/BP/Weapon/AC_Automatic.Shoot` _asac_automatic))))

(event `Key|One`
  (params (Key :type "Key Structure"))
  (bind _ac_pistol (`self.AC_Pistol`))
  (bind _ac_automatic (`self.AC_Automatic`))
  (bind _ac_sniper (`self.AC_Sniper`))
  (bind _ac_pistol_2 (`self.AC_Pistol`))
  ; Chose Weapon
  (:`Pressed`
    (if (or (!= (`self.GunNow`) (`self.AC_Pistol`)) (`self.bHandsIsEmpty`)) :!label _label
      (set `self.bHandsIsEmpty` false)
      (set `self.GunNow` _ac_pistol)
      (`/Engine/EditorBlueprintResources/StandardMacros.IsValid` _ac_pistol
        (:`Is Valid`
          (`SceneComponent.SetVisibility` _ac_pistol true false)
          (`/Engine/EditorBlueprintResources/StandardMacros.IsValid` _ac_automatic
            (:`Is Valid`
              (`SceneComponent.SetVisibility` _ac_automatic false false)
              (`/Engine/EditorBlueprintResources/StandardMacros.IsValid` _ac_sniper
                (:`Is Valid`
                  (`SceneComponent.SetVisibility` _ac_sniper false false)))))))
      (else
        (set `self.bHandsIsEmpty` true)
        (set `self.GunNow` null)
        (`/Engine/EditorBlueprintResources/StandardMacros.IsValid` _ac_pistol_2
          (:`Is Valid`
            (`SceneComponent.SetVisibility` _ac_pistol_2 false false)))))))

(event `Key|NumPadOne`
  (params (Key :type "Key Structure"))
  ; Chose Weapon
  (:`Pressed`
    (goto _label)))

(event `Key|Two`
  (params (Key :type "Key Structure"))
  (bind _ac_pistol (`self.AC_Pistol`))
  (bind _ac_automatic (`self.AC_Automatic`))
  (bind _ac_sniper (`self.AC_Sniper`))
  (bind _ac_automatic_2 (`self.AC_Automatic`))
  ; Chose Weapon
  (:`Pressed`
    (if (or (!= (`self.GunNow`) (`self.AC_Automatic`)) (`self.bHandsIsEmpty`)) :!label _label_2
      (set `self.bHandsIsEmpty` false)
      (set `self.GunNow` _ac_automatic_2)
      (`/Engine/EditorBlueprintResources/StandardMacros.IsValid` _ac_automatic_2
        (:`Is Valid`
          (`SceneComponent.SetVisibility` _ac_automatic_2 true false)
          (`/Engine/EditorBlueprintResources/StandardMacros.IsValid` _ac_pistol
            (:`Is Valid`
              (`SceneComponent.SetVisibility` _ac_pistol false false)
              (`/Engine/EditorBlueprintResources/StandardMacros.IsValid` _ac_sniper
                (:`Is Valid`
                  (`SceneComponent.SetVisibility` _ac_sniper false false)))))))
      (else
        (set `self.bHandsIsEmpty` true)
        (set `self.GunNow` null)
        (`/Engine/EditorBlueprintResources/StandardMacros.IsValid` _ac_automatic
          (:`Is Valid`
            (`SceneComponent.SetVisibility` _ac_automatic false false)))))))

(event `Key|NumPadTwo`
  (params (Key :type "Key Structure"))
  ; Chose Weapon
  (:`Pressed`
    (goto _label_2)))

(event `Key|Three`
  (params (Key :type "Key Structure"))
  (bind _ac_automatic (`self.AC_Automatic`))
  (bind _ac_pistol (`self.AC_Pistol`))
  (bind _ac_sniper (`self.AC_Sniper`))
  (bind _ac_sniper_2 (`self.AC_Sniper`))
  ; Chose Weapon
  (:`Pressed`
    (if (or (!= (`self.GunNow`) (`self.AC_Sniper`)) (`self.bHandsIsEmpty`)) :!label _label_3
      (set `self.bHandsIsEmpty` false)
      (set `self.GunNow` _ac_sniper_2)
      (`/Engine/EditorBlueprintResources/StandardMacros.IsValid` _ac_sniper_2
        (:`Is Valid`
          (`SceneComponent.SetVisibility` _ac_sniper_2 true false)
          (`/Engine/EditorBlueprintResources/StandardMacros.IsValid` _ac_automatic
            (:`Is Valid`
              (`SceneComponent.SetVisibility` _ac_automatic false false)
              (`/Engine/EditorBlueprintResources/StandardMacros.IsValid` _ac_pistol
                (:`Is Valid`
                  (`SceneComponent.SetVisibility` _ac_pistol false false)))))))
      (else
        (set `self.bHandsIsEmpty` true)
        (set `self.GunNow` null)
        (`/Engine/EditorBlueprintResources/StandardMacros.IsValid` _ac_sniper
          (:`Is Valid`
            (`SceneComponent.SetVisibility` _ac_sniper false false)))))))

(event `Key|NumPadThree`
  (params (Key :type "Key Structure"))
  ; Chose Weapon
  (:`Pressed`
    (goto _label_3)))

(fn `AddMappingContext`
  (bind _asplayer_controller (cast `PlayerController` (`self.GetController`)))
  (`EnhancedInputSubsystemInterface.AddMappingContext` (pcsubsystem `EnhancedInputLocalPlayerSubsystem` _asplayer_controller) "/Game/Courses/IA_Courses/NewInputMappingContext.NewInputMappingContext" 0 (struct)))

(fn `MouseControllRotation`
  (bind (_worldlocation _worlddirection) (`PlayerController.DeprojectMousePositionToWorld` (`GameplayStatics.GetPlayerController` 0)))
  (bind (_returnvalue_roll _returnvalue_pitch _returnvalue_yaw) (`KismetMathLibrary.BreakRotator` (`KismetMathLibrary.RInterpTo_Constant` (`self.K2_GetActorRotation`) (`KismetMathLibrary.FindLookAtRotation` (`self.K2_GetActorLocation`) (`.Intersection` (`KismetMathLibrary.LinePlaneIntersection_OriginNormal` _worldlocation (+ _worldlocation (* _worlddirection 10000.0)) (`self.K2_GetActorLocation`) (0.0 0.0 1.0)))) (`GameplayStatics.GetWorldDeltaSeconds`) 720.0)))
  (`Controller.SetControlRotation` (`self.GetController`) (`KismetMathLibrary.MakeRotator` 0.0 0.0 _returnvalue_yaw)))

(fn `Moving`
  (params (InputPin :type "Float (double-precision)") (x :type "Float (double-precision)") (InputPin2 :type "Float (double-precision)") (y :type "Float (double-precision)"))
  (bind _capsulecomponent (`self.CapsuleComponent`))
  (`self.AddMovementInput` (`SceneComponent.GetRightVector` _capsulecomponent) InputPin)
  (`self.AddMovementInput` (`SceneComponent.GetForwardVector` _capsulecomponent) InputPin2))

(fn `UserConstructionScript`)