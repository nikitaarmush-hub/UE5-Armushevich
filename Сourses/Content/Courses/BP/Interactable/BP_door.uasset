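; BP_door is an interactable double door that opens and closes on alternating Interactive events.
; A FlipFlop plays or reverses the DoorOpen timeline, with the DoorMove flag ignoring input until the movement finishes.
; DoorTypes selects whether the timeline alpha slides the two pivots apart, lifts both, or rotates them in opposite directions.
; Slide and lift interpolate from relative locations cached at BeginPlay.
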(event `self.ReceiveBeginPlay`
  (set `self.StartLoc_1` (`SceneComponent.RelativeLocation` (`self.Pivot1`)))
  (set `self.StartLoc_2` (`SceneComponent.RelativeLocation` (`self.Pivot2`))))

(event `/Game/Courses/BP/BPI_Interactive.Interactive`
  (params (Interactor :type "Actor Object Reference"))
  (bind _startloc_1 (`self.StartLoc_1`))
  (bind _startloc_2 (`self.StartLoc_2`))
  (bind _startloc_1_2 (`self.StartLoc_1`))
  (bind _startloc_2_2 (`self.StartLoc_2`))
  (if (not (`self.DoorMove`))
    (set `self.DoorMove` true)
    (`/Engine/EditorBlueprintResources/StandardMacros.FlipFlop`
      (:`A`
        (bind (_direction `_новая_дорожка_1`) (`Timeline|DoorOpen` :!label _label)
          (:`Update`
            (switch `/Game/Courses/BP/Interactable/E_DoorTypes` (`self.DoorTypes`)
              (:`NewEnumerator0`
                (`SceneComponent.K2_SetRelativeLocation` (`self.Pivot1`) (`KismetMathLibrary.VLerp` _startloc_1_2 (+ _startloc_1_2 (`self.SideOffset`)) `_новая_дорожка_1`) false false)
                (`SceneComponent.K2_SetRelativeLocation` (`self.Pivot2`) (`KismetMathLibrary.VLerp` _startloc_2_2 (+ _startloc_2_2 (* (`self.SideOffset`) -1.0)) `_новая_дорожка_1`) false false))
              (:`NewEnumerator1`
                (`SceneComponent.K2_SetRelativeLocation` (`self.Pivot1`) (`KismetMathLibrary.VLerp` _startloc_1 (+ _startloc_1 (`self.UpOffset`)) `_новая_дорожка_1`) false false)
                (`SceneComponent.K2_SetRelativeLocation` (`self.Pivot2`) (`KismetMathLibrary.VLerp` _startloc_2 (+ _startloc_2 (`self.UpOffset`)) `_новая_дорожка_1`) false false))
              (:`NewEnumerator2`
                (`SceneComponent.K2_SetRelativeRotation` (`self.Pivot1`) (`KismetMathLibrary.RLerp` (struct) (`KismetMathLibrary.MakeRotator` 0.0 0.0 (`self.OpenAngle`)) `_новая_дорожка_1`) false false)
                (`SceneComponent.K2_SetRelativeRotation` (`self.Pivot2`) (`KismetMathLibrary.RLerp` (struct) (`KismetMathLibrary.MakeRotator` 0.0 0.0 (* (`self.OpenAngle`) -1.0)) `_новая_дорожка_1`) false false))))
          (:`Finished`
            (set `self.DoorMove` false))))
      (:`B`
        (goto _label :!via `Reverse`)))))

(fn `UserConstructionScript`)