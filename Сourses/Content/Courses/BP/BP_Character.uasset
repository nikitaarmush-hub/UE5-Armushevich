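; BP_Character is a player character for mouse-aimed shooting with Enhanced Input movement along fixed world axes.
; Each Tick intersects the deprojected cursor ray with a horizontal plane at the actor's height and turns control yaw toward that point at a constant rate.
; Left mouse spawns BP_BaseProjecttile at MuzzlePoint, while an alternative line-trace damage shot is left unconnected.
; Debug prints report input, aim point and firing.
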(event `self.ReceiveBeginPlay`
  (bind _asplayer_controller (cast `PlayerController` (`self.GetController`)))
  (`EnhancedInputSubsystemInterface.AddMappingContext` (pcsubsystem `EnhancedInputLocalPlayerSubsystem` _asplayer_controller) "/Game/Courses/AI_Courses/NewInputMappingContext.NewInputMappingContext" 0 (struct)))

(event `EnhancedInput|/Game/Courses/AI_Courses/AI_Move`
  (params (ActionValue :type "Vector2D Structure") (ElapsedSeconds :type "Float (double-precision)") (TriggeredSeconds :type "Float (double-precision)") (InputAction :type "InputAction Object Reference" :default "/Game/Courses/AI_Courses/AI_Move.AI_Move"))
  (:`Triggered`
    (`KismetSystemLibrary.PrintString` (`KismetTextLibrary.Conv_TextToString` (`|FormatText` "X: {x}/ Y: {y}" ActionValue_X ActionValue_Y)))
    (`self.AddMovementInput` (`KismetMathLibrary.GetRightVector` (struct)) ActionValue_X)
    (`self.AddMovementInput` (`KismetMathLibrary.GetForwardVector` (struct)) ActionValue_Y)))

(event `self.ReceiveTick`
  (params (DeltaSeconds :type "Float (single-precision)"))
  (bind (_worldlocation _worlddirection) (`PlayerController.DeprojectMousePositionToWorld` (`GameplayStatics.GetPlayerController` 0)))
  (bind (_t _intersection) (`KismetMathLibrary.LinePlaneIntersection_OriginNormal` _worldlocation (+ _worldlocation (* _worlddirection 10000.0)) (`self.K2_GetActorLocation`) (0.0 0.0 1.0)))
  (bind (_returnvalue_roll _returnvalue_pitch _returnvalue_yaw) (`KismetMathLibrary.BreakRotator` (`KismetMathLibrary.RInterpTo_Constant` (`self.K2_GetActorRotation`) (`KismetMathLibrary.FindLookAtRotation` (`self.K2_GetActorLocation`) _intersection) (`GameplayStatics.GetWorldDeltaSeconds`) 720.0)))
  (`KismetSystemLibrary.PrintString` (`KismetStringLibrary.Conv_VectorToString` _intersection))
  (`Controller.SetControlRotation` (`self.GetController`) (`KismetMathLibrary.MakeRotator` 0.0 0.0 _returnvalue_yaw)))

(event `Key|LeftMouseButton`
  (params (Key :type "Key Structure"))
  (bind (_returnvalue_location _returnvalue_rotation) (`KismetMathLibrary.BreakTransform` (`SceneComponent.K2_GetComponentToWorld` (`self.MuzzlePoint`))))
  (:`Pressed`
    (`KismetSystemLibrary.PrintString` "Fire")
    (`|SpawnActorFromClass` "/Game/Courses/BP/BP_BaseProjecttile.BP_BaseProjecttile_C" (`KismetMathLibrary.MakeTransform` _returnvalue_location _returnvalue_rotation) "Undefined" "MultiplyWithRoot" null null)))

(fn `UserConstructionScript`)