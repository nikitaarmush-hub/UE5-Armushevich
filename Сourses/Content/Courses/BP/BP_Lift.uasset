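; BP_Lift is an elevator actor with Up and Down trigger volumes that light a point light while overlapped and step the platform vertically within roof and floor limits.
; ElevatorUp and ElevatorDawn update the height and call MoveElevator for an eased MoveComponentTo; their ElevatorMove guard clears immediately, since that move is latent.
; Each trigger also counts crossings and shows a random data-table message, one outcome of which can disable player input.
; BeginPlay prints a welcome text plus arithmetic and array-sum results.
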(event `self.ReceiveBeginPlay`
  (bind _returnvalue (`|GetDataTableRow` "/Game/Courses/UI_Table.UI_Table" "Welcome")
    (:`then`
      (`KismetSystemLibrary.PrintText` (`|FormatText` (`.Text_2_FEB23832440420D912199BA6972297CA` (break `/Game/Courses/TextTableRow` _returnvalue))))
      (`self.MathFunct`)
      (`self.ArrayFunct`))))

(event `self.Down.OnComponentBeginOverlap`
  (params (OverlappedComponent :type "PrimitiveComponent Object Reference") (OtherActor :type "Actor Object Reference") (OtherComp :type "PrimitiveComponent Object Reference") (OtherBodyIndex :type Integer) (bFromSweep :type Boolean) (SweepResult :type "HitResult Structure (by ref)"))
  (`SceneComponent.SetVisibility` (`self.PointLight1`) true false)
  (`self.Information`)
  (`self.ElevatorDawn`)
  (`self.CrossTriger` :!label _label)
  (`self.Cross`))

(event `self.Down.OnComponentEndOverlap`
  (params (OverlappedComponent :type "PrimitiveComponent Object Reference") (OtherActor :type "Actor Object Reference") (OtherComp :type "PrimitiveComponent Object Reference") (OtherBodyIndex :type Integer))
  (`SceneComponent.SetVisibility` (`self.PointLight1`) false false))

(event `self.Up.OnComponentBeginOverlap`
  (params (OverlappedComponent :type "PrimitiveComponent Object Reference") (OtherActor :type "Actor Object Reference") (OtherComp :type "PrimitiveComponent Object Reference") (OtherBodyIndex :type Integer) (bFromSweep :type Boolean) (SweepResult :type "HitResult Structure (by ref)"))
  (`SceneComponent.SetVisibility` (`self.PointLight`) true false)
  (`self.Information`)
  (`self.ElevatorUp`)
  (goto _label))

(event `self.Up.OnComponentEndOverlap`
  (params (OverlappedComponent :type "PrimitiveComponent Object Reference") (OtherActor :type "Actor Object Reference") (OtherComp :type "PrimitiveComponent Object Reference") (OtherBodyIndex :type Integer))
  (`SceneComponent.SetVisibility` (`self.PointLight`) false false))

(event `MoveElevator`
  (`KismetSystemLibrary.MoveComponentTo` (`self.Elevator`) (`self.Location`) (struct) true true 3.0)
  (set `self.ElevatorMove` false))

(fn `ArrayFunct`
  (for _array_element (`self.Array`)
    (set `self.Sum` (+ _array_element (`self.Sum`))))
  (`KismetSystemLibrary.PrintText` (`KismetTextLibrary.Conv_IntToText` (`self.Sum`))))

(fn `Cross`
  (bind _returnvalue (`GameplayStatics.GetPlayerController` 0))
  (if (== (`self.TriggerVar`) 3)
    (switch `/Game/Courses/E_Array` "NewEnumerator1"
      (:`NewEnumerator1`
        (`self.DisableInput` (`GameplayStatics.GetPlayerPawn` 0) _returnvalue)
        (`Controller.SetIgnoreMoveInput` _returnvalue true)))))

(fn `CrossTriger`
  (bind _output_get (set `self.HowMuchCross` (+ (`self.HowMuchCross`) 1)))
  (`KismetSystemLibrary.PrintString` (`KismetStringLibrary.Conv_IntToString` _output_get)))

(fn `ElevatorDawn`
  (bind _returnvalue (+ (`self.hight`) (`self.buttonDown`)))
  (if (not (`self.ElevatorMove`))
    (if (not (< (+ (`self.hight`) (`self.buttonDown`)) (`self.flor`)))
      (set `self.ElevatorMove` true)
      (set `self.Location` (`KismetMathLibrary.MakeVector` 0.0 0.0 _returnvalue))
      (`self.MoveElevator`)
      (bind _output_get (set `self.hight` _returnvalue))
      (`KismetSystemLibrary.PrintText` (`KismetTextLibrary.Conv_DoubleToText` _output_get "HalfToEven")))))

(fn `ElevatorUp`
  (bind _returnvalue (+ (`self.hight`) (`self.buttonUp`)))
  (if (not (`self.ElevatorMove`))
    (if (not (> (+ (`self.hight`) (`self.buttonUp`)) (`self.Roof`)))
      (set `self.ElevatorMove` true)
      (set `self.Location` (`KismetMathLibrary.MakeVector` 0.0 0.0 _returnvalue))
      (`self.MoveElevator`)
      (bind _output_get (set `self.hight` _returnvalue))
      (`KismetSystemLibrary.PrintText` (`KismetTextLibrary.Conv_DoubleToText` _output_get "HalfToEven")))))

(fn `Information`
  (bind _output_get (set `self.TriggerVar` (`KismetMathLibrary.RandomIntegerInRange` 2 3)))
  (if (== _output_get 2)
    (bind _returnvalue (`|GetDataTableRow` "/Game/Courses/UI_Table.UI_Table" "W")
      (:`then`
        (`KismetSystemLibrary.PrintText` (`|FormatText` (`.Text_2_FEB23832440420D912199BA6972297CA` (break `/Game/Courses/TextTableRow` _returnvalue))))))
    (else
      (bind _returnvalue_2 (`|GetDataTableRow` "/Game/Courses/UI_Table.UI_Table" "F")
        (:`then`
          (`KismetSystemLibrary.PrintText` (`|FormatText` (`.Text_2_FEB23832440420D912199BA6972297CA` (break `/Game/Courses/TextTableRow` _returnvalue_2)))))))))

(fn `MathFunct`
  (`KismetSystemLibrary.PrintString` (`KismetStringLibrary.Conv_IntToString` (- (/ (* (+ (/ (`self.1Var`) (`self.2Var`)) (`self.3Var`)) (`self.4Var`)) (`self.5Var`)) (`self.6Var`)))))

(fn `UserConstructionScript`)